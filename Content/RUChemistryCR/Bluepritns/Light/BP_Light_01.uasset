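; BP_Light_01 is a configurable lamp fixture that pairs a rect light with two lamp meshes.
; Its construction script applies exposed-style variables for radius, square source size, temperature, barn door length, color and intensity to the RectLight.
; It creates a dynamic material instance per mesh, fixing the first lamp's emissive intensity and driving the second's from a variable.
; The event graph holds no active logic.
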(fn `UserConstructionScript`
  (bind _rectlight (`self.RectLight`))
  (bind _sourse_radius (`self.Sourse Radius`))
  (bind _rectlight_2 (`self.RectLight`))
  (`LocalLightComponent.SetAttenuationRadius` (`self.RectLight`) (`self.Light Radius`))
  (`RectLightComponent.SetSourceWidth` _rectlight _sourse_radius)
  (`RectLightComponent.SetSourceHeight` _rectlight _sourse_radius)
  (`LightComponent.SetTemperature` _rectlight_2 (`self.New Temperature`))
  (`RectLightComponent.SetBarnDoorLength` _rectlight_2 (`self.Barn Length`))
  (`LightComponent.SetLightColor` (`self.RectLight`) (`self.Color`) true)
  (`|ExecutionSequence`
    (:`then_0`
      (bind _returnvalue (`PrimitiveComponent.CreateDynamicMaterialInstance` (`self.SM_Lamp_01`) 0 "/Game/RUChemistryCR/Materials/Substance_MI/MI_Lamp_01.MI_Lamp_01" "None"))
      (set `self.Lamp_Mat 1` _returnvalue))
    (:`then_1`
      (bind _returnvalue_2 (`PrimitiveComponent.CreateDynamicMaterialInstance` (`self.SM_Lamp_02`) 0 "/Game/RUChemistryCR/Materials/Substance_MI/MI_Lamp_02.MI_Lamp_02" "None"))
      (set `self.Lamp_Mat 2` _returnvalue_2))
    (:`then_2`
      (`MaterialInstanceDynamic.SetScalarParameterValue` (`self.Lamp_Mat 1`) "Emissive Intensity" 1.0)
      (`MaterialInstanceDynamic.SetScalarParameterValue` (`self.Lamp_Mat 2`) "Emissive Intensity" (`self.Emissive Intensity`))
      (`LightComponent.SetIntensity` (`self.RectLight`) (`self.Light Intensity`)))))