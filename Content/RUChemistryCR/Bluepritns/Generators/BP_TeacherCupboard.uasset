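; BP_TeacherCupboard is a configurable teacher's cupboard prop with no active runtime logic.
; Its Construction Script uses an Index to pick one of four combinations of small and large cupboard meshes, showing or hiding the matching door pairs.
; It writes hue, desaturation, power and color to Custom Primitive Data on the cupboard and door meshes, allowing per-instance tinting without dynamic material instances.
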(fn `UserConstructionScript`
  (bind _index (`self.Index`))
  (bind _sm_cupboardbig (`self.SM_CupboardBig`))
  (`StaticMeshComponent.SetStaticMesh` (`self.SM_Cupboard`) (select `int` _index :`0` "/Game/RUChemistryCR/Meshes/SM_Cupboard.SM_Cupboard" :`1` "/Game/RUChemistryCR/Meshes/SM_Cupboard02Small.SM_Cupboard02Small" :`2` "/Game/RUChemistryCR/Meshes/SM_Cupboard.SM_Cupboard" :`3` "/Game/RUChemistryCR/Meshes/SM_Cupboard02Small.SM_Cupboard02Small" :!type "StaticMesh Object Reference"))
  (`StaticMeshComponent.SetStaticMesh` (`self.SM_CupboardBig`) (select `int` _index :`0` "/Game/RUChemistryCR/Meshes/SM_CupboardBig.SM_CupboardBig" :`1` "/Game/RUChemistryCR/Meshes/SM_CupboardBig.SM_CupboardBig" :`2` "/Game/RUChemistryCR/Meshes/SM_Cupboard02Large.SM_Cupboard02Large" :`3` "/Game/RUChemistryCR/Meshes/SM_Cupboard02Large.SM_Cupboard02Large" :!type "StaticMesh Object Reference"))
  (`SceneComponent.SetVisibility` (`self.SM_Cupboard02LargeDoor1`) (select `int` (`self.Index`) :`0` false :`1` false :`2` true :`3` true) true)
  (`SceneComponent.SetVisibility` (`self.SM_Cupboard02LargeDoor`) (select `int` (`self.Index`) :`0` false :`1` false :`2` true :`3` true) true)
  (`SceneComponent.SetVisibility` (`self.SM_Cupboard_RightDoor`) (select `int` (`self.Index`) :`0` false :`1` true :`2` false :`3` true) true)
  (`SceneComponent.SetVisibility` (`self.SM_Cupboard_LeftDoor`) (select `int` (`self.Index`) :`0` false :`1` true :`2` false :`3` true) true)
  (`PrimitiveComponent.SetCustomPrimitiveDataFloat` _sm_cupboardbig 0 (`self.HUE`))
  (`PrimitiveComponent.SetCustomPrimitiveDataFloat` (`self.SM_Cupboard_LeftDoor`) 0 (`self.HUE`))
  (`PrimitiveComponent.SetCustomPrimitiveDataFloat` (`self.SM_Cupboard_RightDoor`) 0 (`self.HUE`))
  (`PrimitiveComponent.SetCustomPrimitiveDataFloat` (`self.SM_Cupboard02LargeDoor1`) 0 (`self.HUE`))
  (`PrimitiveComponent.SetCustomPrimitiveDataFloat` (`self.SM_Cupboard02LargeDoor`) 0 (`self.HUE`))
  (`PrimitiveComponent.SetCustomPrimitiveDataFloat` (`self.SM_Cupboard`) 0 (`self.HUE`))
  (`PrimitiveComponent.SetCustomPrimitiveDataFloat` _sm_cupboardbig 1 (`self.DESATURATION`))
  (`PrimitiveComponent.SetCustomPrimitiveDataFloat` (`self.SM_Cupboard02LargeDoor`) 1 (`self.DESATURATION`))
  (`PrimitiveComponent.SetCustomPrimitiveDataFloat` (`self.SM_Cupboard02LargeDoor1`) 1 (`self.DESATURATION`))
  (`PrimitiveComponent.SetCustomPrimitiveDataFloat` (`self.SM_Cupboard`) 1 (`self.DESATURATION`))
  (`PrimitiveComponent.SetCustomPrimitiveDataFloat` (`self.SM_Cupboard_RightDoor`) 1 (`self.DESATURATION`))
  (`PrimitiveComponent.SetCustomPrimitiveDataFloat` (`self.SM_Cupboard_LeftDoor`) 1 (`self.DESATURATION`))
  (`PrimitiveComponent.SetCustomPrimitiveDataFloat` _sm_cupboardbig 2 (`self.POWER`))
  (`PrimitiveComponent.SetCustomPrimitiveDataFloat` (`self.SM_Cupboard02LargeDoor`) 2 (`self.POWER`))
  (`PrimitiveComponent.SetCustomPrimitiveDataFloat` (`self.SM_Cupboard02LargeDoor1`) 2 (`self.POWER`))
  (`PrimitiveComponent.SetCustomPrimitiveDataFloat` (`self.SM_Cupboard`) 2 (`self.POWER`))
  (`PrimitiveComponent.SetCustomPrimitiveDataFloat` (`self.SM_Cupboard_RightDoor`) 2 (`self.POWER`))
  (`PrimitiveComponent.SetCustomPrimitiveDataFloat` (`self.SM_Cupboard_LeftDoor`) 2 (`self.POWER`))
  (`PrimitiveComponent.SetCustomPrimitiveDataVector3` _sm_cupboardbig 3 (`KismetMathLibrary.Conv_LinearColorToVector` (`self.Color`)))
  (`PrimitiveComponent.SetCustomPrimitiveDataVector3` (`self.SM_Cupboard02LargeDoor`) 3 (`KismetMathLibrary.Conv_LinearColorToVector` (`self.Color`)))
  (`PrimitiveComponent.SetCustomPrimitiveDataVector3` (`self.SM_Cupboard02LargeDoor1`) 3 (`KismetMathLibrary.Conv_LinearColorToVector` (`self.Color`)))
  (`PrimitiveComponent.SetCustomPrimitiveDataVector3` (`self.SM_Cupboard`) 3 (`KismetMathLibrary.Conv_LinearColorToVector` (`self.Color`)))
  (`PrimitiveComponent.SetCustomPrimitiveDataVector3` (`self.SM_Cupboard_RightDoor`) 3 (`KismetMathLibrary.Conv_LinearColorToVector` (`self.Color`)))
  (`PrimitiveComponent.SetCustomPrimitiveDataVector3` (`self.SM_Cupboard_LeftDoor`) 3 (`KismetMathLibrary.Conv_LinearColorToVector` (`self.Color`))))