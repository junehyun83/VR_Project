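; VR door Blueprint that a motion controller can grab and swing, with a keyhole lock.
; Grab stores a controller within the hand collision sphere's radius, and Release clears it.
; Tick sets the lock from the keyhole state and the door mesh's world Z position near zero.
; When unlocked, the door's yaw follows the held hand within clamped limits, or snaps shut when released nearly closed.
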(event `/Game/Blueprints/INTERFACE/Grab.Grab`
  (params (MotionController :type "MotionControllerComponent Object Reference"))
  (bind _handcollision (`self.HandCollision`))
  (if (== (`SceneComponent.K2_GetComponentLocation` MotionController) (`SceneComponent.K2_GetComponentLocation` _handcollision) :`ErrorTolerance` (`SphereComponent.SphereRadius` _handcollision))
    (set `self.Hand` MotionController)))

(event `/Game/Blueprints/INTERFACE/Grab.Release`
  (params (MotionController :type "MotionControllerComponent Object Reference"))
  (if (== MotionController (`self.Hand`))
    (set `self.Hand` null)))

(event `self.ReceiveTick`
  (params (DeltaSeconds :type "Float (single-precision)"))
  (bind _hand (`self.Hand`))
  (bind _sm_metal_door_01a (`self.SM_Metal_Door_01a`))
  (bind (_returnvalue_roll _returnvalue_pitch _returnvalue_yaw) (`KismetMathLibrary.BreakRotator` (`SceneComponent.K2_GetComponentRotation` _sm_metal_door_01a)))
  (bind (_returnvalue_x _returnvalue_y _returnvalue_z) (`KismetMathLibrary.BreakVector` (`SceneComponent.K2_GetComponentLocation` (`self.SM_Metal_Door_01a`))))
  (bind (_returnvalue_roll_2 _returnvalue_pitch_2 _returnvalue_yaw_2) (`KismetMathLibrary.BreakRotator` (`KismetMathLibrary.FindLookAtRotation` (`SceneComponent.K2_GetComponentLocation` _hand) (`SceneComponent.K2_GetComponentLocation` _sm_metal_door_01a))))
  (`|ExecutionSequence`
    (:`then_0`
      ;[1 1 1] Locked?
      (if (and (not (`/Game/Blueprints/KeyHole.Unlocked` (`self.KeyHole`))) (`KismetMathLibrary.NearlyEqual_FloatFloat` _returnvalue_z))
        (set `self.Locked` true)
        (else
          (set `self.Locked` false))))
    (:`then_1`
      ;[1 1 1] Set Door Rotation
      (if (not (`self.Locked`))
        (`/Engine/EditorBlueprintResources/StandardMacros.IsValid` _hand
          (:`Is Valid`
            (`SceneComponent.K2_SetWorldRotation` _sm_metal_door_01a (`KismetMathLibrary.MakeRotator` 0.0 0.0 (`KismetMathLibrary.ClampAngle` (- _returnvalue_yaw_2 180.0) -90.0 90.0)) false false))
          (:`Is Not Valid`
            (if (`KismetMathLibrary.NearlyEqual_FloatFloat` _returnvalue_yaw 0.0 10.0)
              (`SceneComponent.K2_SetWorldRotation` :`self` _sm_metal_door_01a))))))))

(event `self.HandCollision.OnComponentBeginOverlap`
  (params (OverlappedComponent :type "PrimitiveComponent Object Reference") (OtherActor :type "Actor Object Reference") (OtherComp :type "PrimitiveComponent Object Reference") (OtherBodyIndex :type Integer) (bFromSweep :type Boolean) (SweepResult :type "HitResult Structure (by ref)")))

(fn `UserConstructionScript`)