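; PowerLever is a lever actor that a motion controller can grab and swing around one axis.
; Grab stores a controller that is within the Sphere's radius, and Release clears it.
; While held, Tick derives an Atan2 angle from the controller direction in LeverPivot's local space and applies it as clamped roll.
; When not held, the pivot snaps to zero rotation only if its roll is already near zero.
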(event `/Game/Blueprints/INTERFACE/Grab.Grab`
  (params (MotionController :type "MotionControllerComponent Object Reference"))
  (bind _sphere (`self.Sphere`))
  (if (== (`SceneComponent.K2_GetComponentLocation` MotionController) (`SceneComponent.K2_GetComponentLocation` _sphere) :`ErrorTolerance` (`SphereComponent.SphereRadius` _sphere))
    (set `self.MotionController` MotionController)))

(event `/Game/Blueprints/INTERFACE/Grab.Release`
  (params (MotionController :type "MotionControllerComponent Object Reference"))
  (if (== MotionController (`self.MotionController`))
    (set `self.MotionController` null)))

(event `self.ReceiveTick`
  (params (DeltaSeconds :type "Float (single-precision)"))
  (bind _leverpivot (`self.LeverPivot`))
  (bind _leverpivot_2 (`self.LeverPivot`))
  (bind _returnvalue_roll (`KismetMathLibrary.BreakRotator` (`SceneComponent.K2_GetComponentRotation` _leverpivot_2)))
  (bind _returnvalue_roll_2 (`KismetMathLibrary.BreakRotator` (`KismetMathLibrary.MakeRotator` (`KismetMathLibrary.FClamp` (`KismetMathLibrary.RadiansToDegrees` (`KismetMathLibrary.Atan2` (.y (`KismetMathLibrary.InverseTransformDirection` (`SceneComponent.K2_GetComponentToWorld` _leverpivot) (`KismetMathLibrary.Normal` (- (`SceneComponent.K2_GetComponentLocation` _leverpivot) (`SceneComponent.K2_GetComponentLocation` (`self.MotionController`))) 1.0))) (.z (`KismetMathLibrary.InverseTransformDirection` (`SceneComponent.K2_GetComponentToWorld` _leverpivot) (`KismetMathLibrary.Normal` (- (`SceneComponent.K2_GetComponentLocation` _leverpivot) (`SceneComponent.K2_GetComponentLocation` (`self.MotionController`))) 1.0))))) -80.0 80.0))))
  (`/Engine/EditorBlueprintResources/StandardMacros.IsValid` (`self.MotionController`)
    (:`Is Valid`
      (`SceneComponent.K2_SetRelativeRotation` (`self.LeverPivot`) (`KismetMathLibrary.MakeRotator` _returnvalue_roll_2) false false))
    (:`Is Not Valid`
      (if (`KismetMathLibrary.NearlyEqual_FloatFloat` _returnvalue_roll 0.0 1.0)
        (`SceneComponent.K2_SetWorldRotation` :`self` _leverpivot_2)))))

(fn `UpdateRotation`)

(fn `UserConstructionScript`)